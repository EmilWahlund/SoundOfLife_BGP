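; SunController drives a day/night cycle by rotating a Sun light and refreshing the sky's sun direction.
; Tick advances time from DeltaSeconds at a fixed rate, or from playback position changes when the assigned sequence matches Sun_Sequence.
; Skip doubles the requested seconds and adds them to TimeOfDay in fixed steps.
; Update converts the hour delta to pitch rotation and fades sun and optional skylight intensity by sun pitch.
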(event `self.ReceiveTick`
  (params (DeltaSeconds :type "Float (single-precision)"))
  (bind _sunsequence (`self.SunSequence`))
  (bind _sequenceplayer (`LevelSequenceActor.SequencePlayer` _sunsequence))
  (bind _returnvalue (- (`MovieSceneSequencePlayer.GetPlaybackPosition` _sequenceplayer) (`self.SequencePreviousTime`)))
  (`/Engine/EditorBlueprintResources/StandardMacros.IsValid` _sunsequence
    (:`Is Valid`
      (if (== _sequenceplayer "/Game/Sequences/Sun_Sequence.Sun_Sequence")
        (`self.Skip` (* _returnvalue (* (/ _returnvalue (`MovieSceneSequencePlayer.GetLength` _sequenceplayer)) 3600.0)))
        (else
          (set `self.SequencePreviousTime` 0.0 :!label _label)
          (`self.Skip` (* DeltaSeconds (/ 180.0 5.0))))))
    (:`Is Not Valid`
      (goto _label))))

(fn `Set Sequence`
  (params (Sequence :type "LevelSequenceActor Object Reference"))
  (set `self.SunSequence` Sequence))

(fn `Skip`
  (params (Seconds :type "Float (double-precision)"))
  (bind _stepsize (`self.StepSize`))
  (bind _output_get (set `self.Seconds` (+ Seconds (`self.Seconds`))))
  (set `self.PreviousTimeOfDay` (`self.TimeOfDay`))
  (while (>= _output_get _stepsize)
    (set `self.Seconds` (- (`self.Seconds`) _stepsize))
    (set `self.TimeOfDay` (+ (`self.TimeOfDay`) (/ 1.0 (/ 3600.0 _stepsize)))))
  (`self.Update`))

(fn `Update`
  (bind _timeofday (`self.TimeOfDay`))
  (bind _previoustimeofday (`self.PreviousTimeOfDay`))
  (bind _skylight (`self.SkyLight`))
  (bind _fadewidth (`self.FadeWidth`))
  (bind _skyfade (`self.SkyFade`))
  (bind (_x _y) (`KismetMathLibrary.BreakVector2D` (`self.SkyIntensity`)))
  (bind _lightcomponent (`Light.LightComponent` (`self.Sun`)))
  ;[1 1 1] deltaHr
  (if (>= _timeofday _previoustimeofday)
    (set `self.deltaHr` (- _timeofday _previoustimeofday))
    (else
      (set `self.deltaHr` (- (+ _timeofday 24.0) _previoustimeofday))))
  ;[1 1 1] Sun Position
  (`self.K2_AddActorLocalRotation` (`self.Sun`) (`KismetMathLibrary.MakeRotator` 0.0 (`KismetMathLibrary.MapRangeUnclamped` (`self.deltaHr`) 0.0 24.0 0.0 360.0)) false false)
  (`/Game/Blueprints/CustomBPSkySphere/BP_Sky_Sphere_Custom.UpdateSunDirection` (`self.Sky`))
  ;[1 1 1] Dim
  (`LightComponent.SetIntensity` _lightcomponent (`KismetMathLibrary.MapRangeClamped` (* (.pitch (`SceneComponent.RelativeRotation` _lightcomponent)) -1.0) (* _fadewidth -1.0) _fadewidth 0.0 (`self.Sun Intensity`)))
  (`/Engine/EditorBlueprintResources/StandardMacros.IsValid` _skylight
    (:`Is Valid`
      (`SkyLightComponent.SetIntensity` (`SkyLight.LightComponent` _skylight) (`KismetMathLibrary.MapRangeClamped` (* (.pitch (`SceneComponent.RelativeRotation` (`Light.LightComponent` (`self.Sun`)))) -1.0) (* _skyfade -1.0) _skyfade _x _y)))))

(fn `UserConstructionScript`)