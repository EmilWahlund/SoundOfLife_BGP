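; Bicycle is a placeable object with configurable steering angle and color, set up entirely in the construction script with no active runtime logic.
; The Front component takes FrontCenter's rotation, then adds a local yaw remapped from Direction, so the front turns either way from center.
; One dynamic instance of the Bike material is applied to both Front and Back, and its Color parameter comes from the Color variable.
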(fn `UserConstructionScript`
  (bind _front (`self.Front`))
  (`SceneComponent.K2_SetRelativeRotation` _front (`SceneComponent.RelativeRotation` (`self.FrontCenter`)) false false)
  (`SceneComponent.K2_AddLocalRotation` _front (`KismetMathLibrary.MakeRotator` 0.0 0.0 (`KismetMathLibrary.MapRangeClamped` (`self.Direction`) 0.0 1.0 -160.0 160.0)) false false)
  (bind _returnvalue (`KismetMaterialLibrary.CreateDynamicMaterialInstance` "/Game/Materials/Textures/Prop_Textures/StreetProps/Bike/Bike.Bike"))
  (`PrimitiveComponent.SetMaterial` (`self.Back`) 0 _returnvalue)
  (`PrimitiveComponent.SetMaterial` (`self.Front`) 0 _returnvalue)
  (`MaterialInstanceDynamic.SetVectorParameterValue` _returnvalue "Color" (`self.Color`)))