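; Work light prop with a static mesh and left and right spot lights, configured once at BeginPlay.
; A dynamic material instance on the mesh's first slot gets its "Light" parameter set from Emissive times Light.
; The same Light multiplier scales LightIntensity for both spot lights, keeping glow and illumination in step.
; The construction script is empty, so this setup applies only when play begins.
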(event `self.ReceiveBeginPlay`
  (bind _staticmesh (`self.StaticMesh`))
  (bind _returnvalue (`PrimitiveComponent.CreateDynamicMaterialInstance` _staticmesh 0 (`PrimitiveComponent.GetMaterial` _staticmesh 0)))
  (`MaterialInstanceDynamic.SetScalarParameterValue` _returnvalue "Light" (* (`self.Emissive`) (`self.Light`)))
  (`LightComponent.SetIntensity` (`self.SpotLight_Left`) (* (`self.LightIntensity`) (`self.Light`)))
  (`LightComponent.SetIntensity` (`self.SpotLight_Right`) (* (`self.LightIntensity`) (`self.Light`))))

(fn `UserConstructionScript`)