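; Modular pipe actor that builds a vertical run of static mesh pieces in the construction script, with no active event logic.
; A loop adds the requested number of segments, stepping the Z offset down by each mesh's local bounds height so pieces stack without hardcoded lengths.
; An extra mesh follows each segment, skipped after the last unless HasBottom is set.
; HasTop and HasBottom toggle the end pieces.
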(fn `UserConstructionScript`
  (bind _returnvalue (- (`self.Segments`) 1))
  (if (`self.HasTop`)
    (`AddComponent|NODE_AddStaticMeshComponent-0`)
    (`AddComponent|NODE_AddStaticMeshComponent-4`))
  (for _index (range (+ _returnvalue 1))
    (bind _returnvalue_2 (`AddComponent|NODE_AddStaticMeshComponent-1` :`RelativeTransform` (`KismetMathLibrary.Conv_VectorToTransform` (`KismetMathLibrary.MakeVector` 0.0 0.0 (`self.Offset`)))))
    (bind (_min _max) (`StaticMeshComponent.GetLocalBounds` _returnvalue_2))
    (bind _output_get (set `self.Offset` (+ (`self.Offset`) (.z (- _min _max)))))
    (if (or (`self.HasBottom`) (!= _index _returnvalue))
      (`AddComponent|NODE_AddStaticMeshComponent-2` :`RelativeTransform` (`KismetMathLibrary.Conv_VectorToTransform` (`KismetMathLibrary.MakeVector` 0.0 0.0 _output_get)))))
  (if (`self.HasBottom`)
    (`AddComponent|NODE_AddStaticMeshComponent-3` :`RelativeTransform` (`KismetMathLibrary.Conv_VectorToTransform` (`KismetMathLibrary.MakeVector` 0.0 0.0 (`self.Offset`))))))