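; Lamp is a placeable light prop that pairs a lamp mesh with a spot light.
; Its construction script creates a dynamic material instance from the bulb material, applies it to the mesh's second slot and sets its emissive parameter.
; The Light value scales both that glow and the spot light's intensity, so the two change together.
; The event graph is empty, so nothing updates at runtime.
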(fn `UserConstructionScript`
  (bind _returnvalue (`KismetMaterialLibrary.CreateDynamicMaterialInstance` "/Game/Meshes/Bar_Props/lampBulb.LampBulb"))
  (`PrimitiveComponent.SetMaterial` (`self.Lamp`) 1 _returnvalue)
  (`MaterialInstanceDynamic.SetScalarParameterValue` _returnvalue "Light" (* (`self.LightEmissive`) (`self.Light`)))
  (`LightComponent.SetIntensity` (`self.SpotLight`) (* (`self.LightIntensity`) (`self.Light`))))