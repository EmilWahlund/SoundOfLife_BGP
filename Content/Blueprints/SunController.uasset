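; Sun controller that drives a time-of-day cycle by moving the sun and refreshing the sky.
; Skip advances TimeOfDay by a given amount, then calls Update.
; Update converts the elapsed hours, allowing for midnight wrap, into an incremental world pitch rotation of the Sun and updates the Sky's sun direction.
; It then fades light intensity from the sun's pitch across a FadeWidth band around the horizon.
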(fn `Skip`
  (params (Amount :type "Float (double-precision)"))
  (bind _timeofday (`self.TimeOfDay`))
  (set `self.PreviousTimeOfDay` _timeofday)
  (set `self.TimeOfDay` (+ Amount _timeofday))
  (`self.Update`))

(fn `Update`
  (bind _timeofday (`self.TimeOfDay`))
  (bind _previoustimeofday (`self.PreviousTimeOfDay`))
  (bind _fadewidth (`self.FadeWidth`))
  (bind _lightcomponent (`Light.LightComponent` (`self.Sun`)))
  ;[1 1 1] deltaHr
  (if (>= _timeofday _previoustimeofday)
    (set `self.deltaHr` (- _timeofday _previoustimeofday))
    (else
      (set `self.deltaHr` (- (+ _timeofday 24.0) _previoustimeofday))))
  ;[1 1 1] Sun Position
  (`self.K2_AddActorWorldRotation` (`self.Sun`) (`KismetMathLibrary.MakeRotator` 0.0 (`KismetMathLibrary.MapRangeUnclamped` (`self.deltaHr`) 0.0 24.0 0.0 360.0)) false false)
  (`/Engine/EngineSky/BP_Sky_Sphere.UpdateSunDirection` (`self.Sky`))
  ;[1 1 1] Dim
  (`LightComponent.SetIntensity` _lightcomponent (`KismetMathLibrary.MapRangeClamped` (* (.pitch (`SceneComponent.RelativeRotation` _lightcomponent)) -1.0) (* _fadewidth -1.0) _fadewidth 0.0 (`self.Sun Intensity`))))

(fn `UserConstructionScript`)