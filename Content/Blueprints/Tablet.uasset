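; Tablet that uses three colour-coded sensors and weight dials to position a listening point for VictimLocation audio sources.
; Each tick clamps weights, rotates dials and, with three sensors placed, moves a particle target to their weighted average position.
; The target spawns only when all sensors lie near their centroid.
; Audio volume follows inverse-square distance from the target, muting when the sensor count drops.
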(event `self.ReceiveTick`
  (params (DeltaSeconds :type "Float (single-precision)"))
  (`|ExecutionSequence`
    (:`then_0`
      (`self.DialUpdate`))
    (:`then_1`
      (`/Engine/EditorBlueprintResources/StandardMacros.IsValid` (`self.Target`)
        (:`Is Valid`
          (bind _count (`self.GetSensorCount`))
          (if (== _count 3)
            (bind _location (`self.GetTargetPosition`))
            (`SceneComponent.K2_SetWorldLocation` (`self.Target`) _location false false)
            (`self.SetAudio`)
            (else
              (`ActorComponent.K2_DestroyComponent` (`self.Target`))
              (`self.KillAudio`))))
        (:`Is Not Valid`
          (bind _count_2 (`self.GetSensorCount`))
          (if (== _count_2 3)
            (bind (_location_2 _isproximity) (`self.GetTargetPosition`))
            (if _isproximity
              (bind _returnvalue (`GameplayStatics.SpawnEmitterAtLocation` "/Game/Particles/SensorTarget_P.SensorTarget_P" _location_2))
              (set `self.Target` _returnvalue)
              (`self.GetAllAudio`)
              (`self.SetAudio`))))))))

(fn `AdjustDial`
  (params (index :type Integer) (amount :type "Float (double-precision)"))
  (switch `int` index
    (:`0`
      (set `self.weight_Sensor_0` (+ (`self.weight_Sensor_0`) amount)))
    (:`1`
      (set `self.weight_Sensor_1` (+ (`self.weight_Sensor_1`) amount)))
    (:`2`
      (set `self.weight_Sensor_2` (+ (`self.weight_Sensor_2`) amount)))))

(fn `Assign Sensor`
  (params (Sensor :type "Sensor Object Reference"))
  (`/Engine/EditorBlueprintResources/StandardMacros.IsValid` (`self.Sensor_0`)
    (:`Is Valid`
      (`/Engine/EditorBlueprintResources/StandardMacros.IsValid` (`self.Sensor_1`)
        (:`Is Valid`
          (`/Engine/EditorBlueprintResources/StandardMacros.IsValid` (`self.Sensor_2`)
            (:`Is Not Valid`
              (bind _output_get (set `self.Sensor_2` Sensor))
              (`MeshComponent.SetVectorParameterValueOnMaterials` (`Sensor.mesh` _output_get) "LightColor" (0.0 0.0 35.0)))))
        (:`Is Not Valid`
          (bind _output_get_2 (set `self.Sensor_1` Sensor))
          (`MeshComponent.SetVectorParameterValueOnMaterials` (`Sensor.mesh` _output_get_2) "LightColor" (0.0 35.0 0.0)))))
    (:`Is Not Valid`
      (bind _output_get_3 (set `self.Sensor_0` Sensor))
      (`MeshComponent.SetVectorParameterValueOnMaterials` (`Sensor.mesh` _output_get_3) "LightColor" (35.0 0.0 0.0)))))

(fn `DestroyAllSensors`
  (bind _sensor_0 (`self.Sensor_0`))
  (bind _sensor_1 (`self.Sensor_1`))
  (bind _sensor_2 (`self.Sensor_2`))
  (`|ExecutionSequence`
    (:`then_0`
      (`/Engine/EditorBlueprintResources/StandardMacros.IsValid` _sensor_0
        (:`Is Valid`
          (`self.K2_DestroyActor` _sensor_0))))
    (:`then_1`
      (`/Engine/EditorBlueprintResources/StandardMacros.IsValid` _sensor_1
        (:`Is Valid`
          (`self.K2_DestroyActor` _sensor_1))))
    (:`then_2`
      (`/Engine/EditorBlueprintResources/StandardMacros.IsValid` _sensor_2
        (:`Is Valid`
          (`self.K2_DestroyActor` _sensor_2))))))

(fn `DialUpdate`
  (set `self.weight_Sensor_0` (`KismetMathLibrary.FClamp` (`self.weight_Sensor_0`) 0.0 2.0))
  (set `self.weight_Sensor_1` (`KismetMathLibrary.FClamp` (`self.weight_Sensor_1`) 0.0 2.0))
  (set `self.weight_Sensor_2` (`KismetMathLibrary.FClamp` (`self.weight_Sensor_2`) 0.0 2.0))
  (`SceneComponent.K2_SetWorldRotation` (`self.Dial_0`) (`KismetMathLibrary.RLerp` (`SceneComponent.K2_GetComponentRotation` (`self.Dial_Min`)) (`SceneComponent.K2_GetComponentRotation` (`self.Dial_Max`)) (/ (`self.weight_Sensor_0`) 2.0) true) false false)
  (`SceneComponent.K2_SetWorldRotation` (`self.Dial_1`) (`KismetMathLibrary.RLerp` (`SceneComponent.K2_GetComponentRotation` (`self.Dial_Min`)) (`SceneComponent.K2_GetComponentRotation` (`self.Dial_Max`)) (/ (`self.weight_Sensor_1`) 2.0) true) false false)
  (`SceneComponent.K2_SetWorldRotation` (`self.Dial_2`) (`KismetMathLibrary.RLerp` (`SceneComponent.K2_GetComponentRotation` (`self.Dial_Min`)) (`SceneComponent.K2_GetComponentRotation` (`self.Dial_Max`)) (/ (`self.weight_Sensor_2`) 2.0) true) false false))

(fn `GetAllAudio`
  (bind _outactors (`GameplayStatics.GetAllActorsOfClass` "/Script/SoundOfLife_BGP.VictimLocation"))
  (bind _output_get (set `self.AudioSources` _outactors))
  (for _ _output_get
    _))

(fn `GetSensorCount`
  (returns (Count :type Integer))
  (bind _output_get (set `self.Count` 0))
  (`/Engine/EditorBlueprintResources/StandardMacros.IsValid` (`self.Sensor_0`)
    (:`Is Valid`
      (bind _result (`/Engine/EditorBlueprintResources/StandardMacros.IncrementInt` _output_get)
        (:`  `
          _)))
    (:`Is Not Valid`
      _))
  (`/Engine/EditorBlueprintResources/StandardMacros.IsValid` (`self.Sensor_1`)
    (:`Is Valid`
      (bind _result_2 (`/Engine/EditorBlueprintResources/StandardMacros.IncrementInt` _result)
        (:`  `
          _)))
    (:`Is Not Valid`
      _))
  (`/Engine/EditorBlueprintResources/StandardMacros.IsValid` (`self.Sensor_2`)
    (:`Is Valid`
      (bind _result_3 (`/Engine/EditorBlueprintResources/StandardMacros.IncrementInt` _result_2)
        (:`  `
          _)))
    (:`Is Not Valid`
      _))
  (return _result_3))

(fn `GetTargetPosition`
  (returns (Location :type "Vector Structure") (isProximity :type Boolean))
  (bind _proximitycheck (`self.proximityCheck`))
  (bind _weight_sensor_0 (`self.weight_Sensor_0`))
  (bind _weight_sensor_1 (`self.weight_Sensor_1`))
  (bind _weight_sensor_2 (`self.weight_Sensor_2`))
  (bind _returnvalue (`self.K2_GetActorLocation` (`self.Sensor_2`)))
  (bind _returnvalue_2 (`self.K2_GetActorLocation` (`self.Sensor_0`)))
  (bind _returnvalue_3 (`self.K2_GetActorLocation` (`self.Sensor_1`)))
  (bind _returnvalue_4 (/ (+ _weight_sensor_0 _weight_sensor_1 _weight_sensor_2) 3.0))
  (bind _returnvalue_5 (/ (+ _returnvalue_2 _returnvalue_3 _returnvalue) 3.0))
  (return (/ (+ (* (`self.K2_GetActorLocation` (`self.Sensor_0`)) (/ _weight_sensor_0 _returnvalue_4)) (* (`self.K2_GetActorLocation` (`self.Sensor_1`)) (/ _weight_sensor_1 _returnvalue_4)) (* (`self.K2_GetActorLocation` (`self.Sensor_2`)) (/ _weight_sensor_2 _returnvalue_4))) 3.0) (and (> _proximitycheck (`KismetMathLibrary.VSize` (- _returnvalue_2 _returnvalue_5))) (> _proximitycheck (`KismetMathLibrary.VSize` (- _returnvalue_5 _returnvalue_3))) (> _proximitycheck (`KismetMathLibrary.VSize` (- _returnvalue_5 _returnvalue))))))

(fn `KillAudio`
  (for _array_element (`self.AudioSources`)
    (`VictimLocation.SetVolume` _array_element 0.0)))

(fn `SetAudio`
  (for _array_element (`self.AudioSources`)
    (`VictimLocation.SetVolume` _array_element (`KismetMathLibrary.FClamp` (/ (* (`self.volumeAtOneMeter`) 10000.0) (`KismetMathLibrary.Square` (`KismetMathLibrary.VSize` (- (`self.K2_GetActorLocation` _array_element) (`SceneComponent.K2_GetComponentLocation` (`self.Target`)))))) 0.0 3.0))))

(fn `UserConstructionScript`)