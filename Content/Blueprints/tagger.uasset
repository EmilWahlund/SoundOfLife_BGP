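; Editor-time helper Blueprint that tags debris actors and their components in the level, with no active runtime logic.
; Its construction script resets a Refresh flag, then scans every actor for "ebris" in the object name.
; Matches whose first tag isn't "debris" get that tag appended, and only then are their components tagged, skipping any already tagged first as "debris".
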(fn `UserConstructionScript`
  (set `self.Refresh` false)
  (bind _outactors (`GameplayStatics.GetAllActorsOfClass` "/Script/Engine.Actor"))
  (for _array_element _outactors
    (if (`KismetStringLibrary.Contains` (`KismetSystemLibrary.GetObjectName` _array_element) "ebris")
      (bind _tags (`Actor.Tags` _array_element))
      (if (!= (`KismetArrayLibrary.Array_Get` _tags) "debris")
        (`KismetArrayLibrary.Array_Add` _tags "debris")
        (for _array_element_2 (`self.K2_GetComponentsByClass` _array_element "/Script/Engine.ActorComponent")
          (bind _componenttags (`ActorComponent.ComponentTags` _array_element_2))
          (if (or (== (`KismetArrayLibrary.Array_Length` _componenttags) 0) (!= (`KismetArrayLibrary.Array_Get` _componenttags) "debris"))
            (`KismetArrayLibrary.Array_Add` _componenttags "debris")))))))