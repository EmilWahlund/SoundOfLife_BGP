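; Particle controller Blueprint that makes a falling dust effect fire in intermittent bursts.
; On BeginPlay it seeds a timer with a random delay drawn from the DelayRange vector.
; Tick counts the timer down and, at zero, sends a "Burst" particle event at the ParticleSystem component's world location, then picks a new random delay.
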(event `self.ReceiveBeginPlay`
  (bind (_x _y) (`KismetMathLibrary.BreakVector2D` (`self.DelayRange`)))
  (set `self.Timer` (`KismetMathLibrary.RandomFloatInRange` _x _y)))

(event `self.ReceiveTick`
  (params (DeltaSeconds :type "Float (single-precision)"))
  (bind _particlesystem (`self.ParticleSystem`))
  (bind (_x _y) (`KismetMathLibrary.BreakVector2D` (`self.DelayRange`)))
  (bind _output_get (set `self.Timer` (- (`self.Timer`) DeltaSeconds)))
  (if (<= _output_get 0.0)
    (`ParticleSystemComponent.GenerateParticleEvent` _particlesystem "Burst" 0.0 (`SceneComponent.K2_GetComponentLocation` _particlesystem) (0.0 0.0 0.0) (0.0 0.0 0.0))
    (set `self.Timer` (`KismetMathLibrary.RandomFloatInRange` _x _y))))

(fn `UserConstructionScript`)